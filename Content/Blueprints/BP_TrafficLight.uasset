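; BP_TrafficLight is a traffic light with Red, Yellow and Green lamp components that light up one colour on request.
; The ColorControl event takes a colour and a duration, swaps that lamp's material to its lit version, waits, then restores the shared M_TrafficColor material.
; It has no sequencing of its own, as BeginPlay and the construction script are empty, so ColorControl must be triggered from outside.
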(event Custom|ColorControl
  (params (Color :type E_LightColor%20Enum :default "NewEnumerator0") (Timer :type Float%20%28double-precision%29))
  (Variables|Default|SetTimer Timer)
  (switch Utilities|FlowControl|Switch|SwitchonE_LightColor Color
    (:NewEnumerator0
      (Rendering|Material|SetMaterial (Variables|Default|GetRed) 0 "/Game/Materials/M_red.M_red")
      (Utilities|FlowControl|Delay (Variables|Default|GetTimer))
      (Rendering|Material|SetMaterial (Variables|Default|GetRed) 0 "/Game/Blueprints/Materials/M_TrafficColor.M_TrafficColor"))
    (:NewEnumerator1
      (Rendering|Material|SetMaterial (Variables|Default|GetYellow) 0 "/Game/Materials/M_Yellow.M_Yellow")
      (Utilities|FlowControl|Delay (Variables|Default|GetTimer))
      (Rendering|Material|SetMaterial (Variables|Default|GetYellow) 0 "/Game/Blueprints/Materials/M_TrafficColor.M_TrafficColor"))
    (:NewEnumerator2
      (Rendering|Material|SetMaterial (Variables|Default|GetGreen) 0 "/Game/Materials/M_Green.M_Green")
      (Utilities|FlowControl|Delay (Variables|Default|GetTimer))
      (Rendering|Material|SetMaterial (Variables|Default|GetGreen) 0 "/Game/Blueprints/Materials/M_TrafficColor.M_TrafficColor"))))

(event EventBeginPlay)

(fn ConstructionScript)