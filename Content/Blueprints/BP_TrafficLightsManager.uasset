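; Manager that finds all BP_TrafficLight actors at BeginPlay and animates them as two signal groups cycling in opposite order.
; The first three found form one group, the rest the other, which starts both loops on reaching three.
; Delayed ForEach loops light each lamp from the ColorSettings map, hold it per color, then black it out, reversing the array each pass.
; Delay variants zero one color's hold on return passes; disconnected test logic remains.
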(event Custom|Recolor
  (bind _trafficlight2 (Variables|Default|GetTrafficLight2))
  (bind _trafficlight1 (Variables|Default|GetTrafficLight1))
  (bind _trafficlight2_2 (Variables|Default|GetTrafficLight2))
  (bind _trafficlight2_3 (Variables|Default|GetTrafficLight2))
  (bind _trafficlight1_2 (Variables|Default|GetTrafficLight1))
  (bind _outactors (Actor|GetAllActorsOfClass "/Game/Blueprints/BP_TrafficLight.BP_TrafficLight_C"))
  (for _array_element _outactors
    (if (< (Utilities|Array|Length _trafficlight1_2) 3)
      (Utilities|Array|Add _trafficlight1_2 _array_element)
      (else
        (Utilities|Array|Add _trafficlight2 _array_element)
        (if (== (Utilities|Array|Length _trafficlight2) 3)
          (Utilities|FlowControl|Sequence
            (:then_0
              (bind _array_element_2 (Utilities|ForEachLoopwithDelay (Variables|Default|GetTrafficLight1) :!label _label)
                (:LoopBody
                  (Default|ChangeColor _array_element_2 (.Value (Utilities|Map|Find (.colormap (Variables|Default|GetColorSettings)) (Variables|/Game/Blueprints/BP_TrafficLight.BP_TrafficLight_C|GetLightColor _array_element_2)))))
                (:Completed
                  (Utilities|Array|Reverse _trafficlight1)
                  (bind _array_element_3 (Utilities|ForEachLoopwithDelay _trafficlight1 :!label _label_2)
                    (:LoopBody
                      (Default|ChangeColor _array_element_3 (.Value (Utilities|Map|Find (.colormap (Variables|Default|GetColorSettings)) (Variables|/Game/Blueprints/BP_TrafficLight.BP_TrafficLight_C|GetLightColor _array_element_3)))))
                    (:Completed
                      (Utilities|Array|Reverse _trafficlight1)
                      (goto _label))
                    (:ToDelay
                      (Utilities|Delay1 (Variables|/Game/Blueprints/BP_TrafficLight.BP_TrafficLight_C|GetLightColor _array_element_3) (Variables|/Game/Blueprints/BP_TrafficLight.BP_TrafficLight_C|GetLightColor _array_element_3) (Variables|/Game/Blueprints/BP_TrafficLight.BP_TrafficLight_C|GetLightColor _array_element_3))
                      (Default|ChangeColor _array_element_3)
                      (goto _label_2 FromDelay))))
                (:ToDelay
                  (Utilities|Delay (Variables|/Game/Blueprints/BP_TrafficLight.BP_TrafficLight_C|GetLightColor _array_element_2) (Variables|/Game/Blueprints/BP_TrafficLight.BP_TrafficLight_C|GetLightColor _array_element_2) (Variables|/Game/Blueprints/BP_TrafficLight.BP_TrafficLight_C|GetLightColor _array_element_2))
                  (Default|ChangeColor _array_element_2)
                  (goto _label FromDelay))))
            (:then_1
              (Utilities|Array|Reverse _trafficlight2_3)
              (bind _array_element_4 (Utilities|ForEachLoopwithDelay _trafficlight2_3 :!label _label_3)
                (:LoopBody
                  (Default|ChangeColor _array_element_4 (.Value (Utilities|Map|Find (.colormap (Variables|Default|GetColorSettings)) (Variables|/Game/Blueprints/BP_TrafficLight.BP_TrafficLight_C|GetLightColor _array_element_4)))))
                (:Completed
                  (Utilities|Array|Reverse _trafficlight2_2)
                  (bind _array_element_5 (Utilities|ForEachLoopwithDelay _trafficlight2_2 :!label _label_4)
                    (:LoopBody
                      (Default|ChangeColor _array_element_5 (.Value (Utilities|Map|Find (.colormap (Variables|Default|GetColorSettings)) (Variables|/Game/Blueprints/BP_TrafficLight.BP_TrafficLight_C|GetLightColor _array_element_5)))))
                    (:Completed
                      (Utilities|Array|Reverse _trafficlight2_2)
                      (goto _label_3))
                    (:ToDelay
                      (Utilities|Delay0 (Variables|/Game/Blueprints/BP_TrafficLight.BP_TrafficLight_C|GetLightColor _array_element_5) (Variables|/Game/Blueprints/BP_TrafficLight.BP_TrafficLight_C|GetLightColor _array_element_5) (Variables|/Game/Blueprints/BP_TrafficLight.BP_TrafficLight_C|GetLightColor _array_element_5))
                      (Default|ChangeColor _array_element_5)
                      (goto _label_4 FromDelay))))
                (:ToDelay
                  (Utilities|Delay (Variables|/Game/Blueprints/BP_TrafficLight.BP_TrafficLight_C|GetLightColor _array_element_4) (Variables|/Game/Blueprints/BP_TrafficLight.BP_TrafficLight_C|GetLightColor _array_element_4) (Variables|/Game/Blueprints/BP_TrafficLight.BP_TrafficLight_C|GetLightColor _array_element_4))
                  (Default|ChangeColor _array_element_4)
                  (goto _label_3 FromDelay))))))))))

(event EventBeginPlay
  (CallFunction|Recolor))

(fn ConstructionScript)